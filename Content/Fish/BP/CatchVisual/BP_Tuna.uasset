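; BP_Tuna is a tuna catch visual that flies along an arc to a target location, then despawns with an effect.
; StartFlight stores the target and the actor's current location, then plays a timeline.
; The timeline's Alpha lerps between the two points while its HeightArc curve adds a scaled vertical offset, and finishing calls PlayDespawnEffect.
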(event `self.StartFlight`
  (params (TargetLocation :type "Vector Structure"))
  (`|ExecutionSequence`
    (:`then_0`
      (bind _output_get (set `self.TargetLoc` TargetLocation))
      (bind (_direction _alpha _heightarc) (`Timeline|Timeline`)
        (:`Update`
          (`self.K2_SetActorLocation` (+ (`KismetMathLibrary.MakeVector` 0.0 0.0 (* _heightarc 300.0)) (`KismetMathLibrary.VLerp` (stale _output_get_2) _output_get _alpha))))
        (:`Finished`
          (`self.PlayDespawnEffect`))))
    (:`then_1`
      (bind _output_get_2 (set `self.StartLoc` (`self.K2_GetActorLocation`))))))

(fn `UserConstructionScript`)